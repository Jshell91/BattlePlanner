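; MyUnit is a unit Blueprint that holds the stats of a single game unit.
; SetVariables copies a UnitData input into member variables covering identity, faction, tier, cost, class, command, range, movement, attack, protection and abilities.
; The event graph and construction script are empty, so the Blueprint acts as a data holder with no behavior of its own.
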(event EventBeginPlay)

(event Collision|EventActorBeginOverlap
  (params (OtherActor :type Actor%20Object%20Reference)))

(event EventTick
  (params (DeltaSeconds :type Float%20%28single-precision%29)))

(fn ConstructionScript)

(fn SetVariables
  (params (UnitData :type Unit%20Data%20Structure))
  (bind (_name _faction _tier _resource _cost _class _command _range _movement _atklight _atkheavy _protection _abilities) (Utilities|Struct|BreakUnitData UnitData))
  (Variables|Default|Setname _name)
  (Variables|Default|Setfaction _faction)
  (Variables|Default|Settier _tier)
  (Variables|Default|Setresource _resource)
  (Variables|Default|Setcost _cost)
  (Variables|Default|SetClass _class)
  (Variables|Default|Setcommand _command)
  (Variables|Default|Setrange _range)
  (Variables|Default|Setmovement _movement)
  (Variables|Default|Setatklight _atklight)
  (Variables|Default|Setatkheavy _atkheavy)
  (Variables|Default|Setprotection _protection)
  (Variables|Default|SetAbility _abilities))