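; MyTile is a tile actor that stores its coordinates, its size and separate light and heavy movement costs.
; On BeginPlay it caches SizeX and SizeY from the maximum X and Y of its static mesh's bounding box.
; Two setter functions, SetCoordinates and SetMovementCost, assign the coordinates and both costs, while the construction script, overlap and Tick do nothing.
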(event EventBeginPlay
  (bind _staticmesh (Variables|Default|GetStaticMesh))
  (bind _staticmesh_2 (Variables|/Script/Engine.StaticMeshComponent|GetStaticMesh _staticmesh))
  (bind _returnvalue (StaticMesh|GetBoundingBox _staticmesh_2))
  (bind _max (Utilities|Struct|BreakBox _returnvalue))
  (bind (_x _y) (Math|Vector|BreakVector _max))
  (Variables|Default|Setsize_x _x)
  (Variables|Default|Setsize_y _y))

(event Collision|EventActorBeginOverlap
  (params (OtherActor :type Actor%20Object%20Reference)))

(event EventTick
  (params (DeltaSeconds :type Float%20%28single-precision%29)))

(fn ConstructionScript)

(fn SetMovementCost
  (params (Light :type Integer) (Heavy :type Integer))
  (Variables|Default|Setlightmovecost Light)
  (Variables|Default|Setheavymovecost Heavy))

(fn SetCoordinates
  (params (CoX :type Integer) (CoY :type Integer))
  (Variables|Default|Setco_x CoX)
  (Variables|Default|Setco_y CoY))