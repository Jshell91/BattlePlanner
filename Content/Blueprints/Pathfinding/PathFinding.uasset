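; Pathfinding Blueprint that computes tile paths for units on a battle map.
; It holds several iterations: A*-style searches using open/closed sets, G/H/F costs and parent links, plus FindPath5, a greedy walk toward the neighbour nearest the target.
; GetDistance weights world distance by the destination tile's Light or Heavy move cost, with grid-coordinate and unweighted variants alongside.
; Some searches rebuild the route through RetracePath, while others return an accumulated array.
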(event EventBeginPlay)

(event Collision|EventActorBeginOverlap
  (params (OtherActor :type Actor%20Object%20Reference)))

(event EventTick
  (params (DeltaSeconds :type Float%20%28single-precision%29)))

(fn ConstructionScript)

(fn FindPath
  (params (Start :type My%20Tile%20Object%20Reference) (Target :type My%20Tile%20Object%20Reference))
  (bind _openset (Variables|Default|GetOpenSet))
  (bind _openset_2 (Variables|Default|GetOpenSet))
  (bind _returnvalue (Utilities|Array|Length _openset))
  (Variables|Default|SetTarget Target)
  (Utilities|Array|Add _openset Start)
  (while (> _returnvalue 0)
    (bind _output_get (Variables|Default|SetCurrent (Utilities|Array|Get(acopy) _openset)))
    ;[1 1 1] ForLoop to check the lowest FCost
    (for _index (range 1 _returnvalue)
      (bind _fcost (Default|FCostCalc (Utilities|Array|Get(acopy) _openset _index)))
      (bind _fcost_2 (Default|FCostCalc _output_get))
      (if (and (<= _fcost _fcost_2) (< (Variables|/Game/Blueprints/MyTile.MyTile_C|GethCost _output_get) (Variables|/Game/Blueprints/MyTile.MyTile_C|GethCost (Utilities|Array|Get(acopy) _openset _index))))
        (Variables|Default|SetCurrent (Utilities|Array|Get(acopy) _openset _index))))
    (Utilities|Array|RemoveItem _openset (Variables|Default|GetCurrent))
    (Utilities|Array|Add (Variables|Default|GetCloseSet) (Variables|Default|GetCurrent))
    (if (== (Variables|Default|GetCurrent) (Variables|Default|GetTarget))
      (bind _endpath (CallFunction|RetracePath Start (Variables|Default|GetTarget)))
      (return _endpath)
      (else
        (bind _outactors (Actor|GetAllActorsOfClass "/Game/Blueprints/MyBattleMap.MyBattleMap_C"))
        (bind _neighbours (Default|GetNeighbours (Utilities|Array|Get(acopy) _outactors) (Variables|Default|GetCurrent)))
        (for _array_element _neighbours
          (bind _distance (CallFunction|GetDistance (Variables|Default|GetCurrent) _array_element))
          (bind _output_get_2 (LocalVariables|SetMoveCost (+ (Variables|/Game/Blueprints/MyTile.MyTile_C|GetgCost (Variables|Default|GetCurrent)) _distance)))
          (if (or (< _output_get_2 (Variables|/Game/Blueprints/MyTile.MyTile_C|GetgCost _array_element)) (not (Utilities|Array|ContainsItem (Variables|Default|GetOpenSet) _array_element)))
            (Variables|/Game/Blueprints/MyTile.MyTile_C|SetgCost _array_element _output_get_2)
            (bind _distance_2 (CallFunction|GetDistance _array_element (Variables|Default|GetTarget)))
            (Variables|/Game/Blueprints/MyTile.MyTile_C|SethCost _array_element _distance_2)
            (Variables|/Game/Blueprints/MyTile.MyTile_C|SetParent _array_element (Variables|Default|GetCurrent))
            (if (not (Utilities|Array|ContainsItem _openset_2 _array_element))
              (Utilities|Array|Add _openset_2 _array_element))))))))

(fn GetDistance
  (params (TileA :type My%20Tile%20Object%20Reference) (TileB :type My%20Tile%20Object%20Reference))
  (switch Utilities|FlowControl|Switch|SwitchonEClass (Variables|/Script/BattlePlanner.Unit|GetClass (Variables|Default|GetUnit))
    (:light
      (return (* (Math|Float|Truncate (Math|Vector|Distance(Vector) (Transformation|GetWorldLocation (Variables|/Game/Blueprints/MyTile.MyTile_C|GetStaticMesh TileA)) (Transformation|GetWorldLocation (Variables|/Game/Blueprints/MyTile.MyTile_C|GetStaticMesh TileB)))) (Variables|/Script/BattlePlanner.Tile|Getlightmovecost TileB))))
    (:heavy
      (return (* (Variables|/Script/BattlePlanner.Tile|Getheavymovecost TileB) (Math|Float|Truncate (Math|Vector|Distance(Vector) (Transformation|GetWorldLocation (Variables|/Game/Blueprints/MyTile.MyTile_C|GetStaticMesh TileA)) (Transformation|GetWorldLocation (Variables|/Game/Blueprints/MyTile.MyTile_C|GetStaticMesh TileB)))))))))

(fn RetracePath
  (params (Start :type My%20Tile%20Object%20Reference) (End :type My%20Tile%20Object%20Reference))
  (bind _reversed (LocalVariables|GetReversed))
  (bind _path (LocalVariables|GetPath))
  (LocalVariables|SetLCurrent End)
  (while (!= (LocalVariables|GetLCurrent) Start)
    (if (not (Utilities|Array|ContainsItem _path (LocalVariables|GetLCurrent)))
      (Utilities|Array|Add _path (LocalVariables|GetLCurrent))
      (LocalVariables|SetLCurrent (Variables|/Game/Blueprints/MyTile.MyTile_C|GetParent (LocalVariables|GetLCurrent)))))
  (bind _arrayelement (Utilities|Array|ReverseforEachLoop (LocalVariables|GetPath))
    (:LoopBody
      (Utilities|Array|Add _reversed _arrayelement))
    (:Completed
      (return _reversed))))

(fn GCostCalc
  (params (Current :type My%20Tile%20Object%20Reference) (Start :type My%20Tile%20Object%20Reference))
  (bind _distance (CallFunction|GetDistance Current Start))
  (Variables|/Game/Blueprints/MyTile.MyTile_C|SetgCost Current _distance))

(fn HCostCalc
  (params (Current :type My%20Tile%20Object%20Reference) (Target :type My%20Tile%20Object%20Reference))
  (bind _distance (CallFunction|GetDistance Current Target))
  (Variables|/Game/Blueprints/MyTile.MyTile_C|SethCost Current _distance))

(fn FCostCalc
  (params (Current :type My%20Tile%20Object%20Reference)))

(fn FindPath2
  (params (Start :type My%20Tile%20Object%20Reference) (Target :type My%20Tile%20Object%20Reference))
  (bind _lopenset (LocalVariables|GetLOpenSet))
  (bind _returnvalue (Utilities|Array|Length _lopenset))
  (Utilities|Array|Add _lopenset Start)
  (while (> _returnvalue 0)
    (bind _output_get (LocalVariables|SetNode (Utilities|Array|Get(acopy) _lopenset)))
    (for _index (range 1 _returnvalue)
      (if (<= (Variables|/Game/Blueprints/MyTile.MyTile_C|GetfCost (Utilities|Array|Get(acopy) _lopenset _index)) (Variables|/Game/Blueprints/MyTile.MyTile_C|GetfCost _output_get))
        (if (< (Variables|/Game/Blueprints/MyTile.MyTile_C|GethCost (Utilities|Array|Get(acopy) _lopenset _index)) (Variables|/Game/Blueprints/MyTile.MyTile_C|GethCost _output_get))
          (LocalVariables|SetNode (Utilities|Array|Get(acopy) _lopenset _index))))
      (Utilities|Array|RemoveItem (LocalVariables|GetLOpenSet) (LocalVariables|GetNode))
      (Utilities|Array|Add (LocalVariables|GetLCloseSet) (LocalVariables|GetNode))
      (if (== (LocalVariables|GetNode) Target)
        (return 0)
        (else
          (bind _outactors (Actor|GetAllActorsOfClass "/Game/Blueprints/MyBattleMap.MyBattleMap_C"))
          (bind _neighbours (Default|GetNeighbours2 (Utilities|Array|Get(acopy) _outactors) (LocalVariables|GetNode)))
          (for _array_element _neighbours
            (bind _distance (CallFunction|GetDistance (LocalVariables|GetNode) _array_element))
            (bind _output_get_2 (LocalVariables|SetMoveCost (+ (Variables|/Game/Blueprints/MyTile.MyTile_C|GetgCost (LocalVariables|GetNode)) _distance)))
            (if (or (< _output_get_2 (Variables|/Game/Blueprints/MyTile.MyTile_C|GetgCost _array_element)) (not (Utilities|Array|ContainsItem (LocalVariables|GetLOpenSet) _array_element)))
              (Variables|/Game/Blueprints/MyTile.MyTile_C|SetgCost _array_element _output_get_2)
              (bind _distance_2 (CallFunction|GetDistance (LocalVariables|GetNode) _array_element))
              (Variables|/Game/Blueprints/MyTile.MyTile_C|SethCost _array_element _distance_2)
              (Variables|/Game/Blueprints/MyTile.MyTile_C|SetParent _array_element (LocalVariables|GetNode))
              (if (not (Utilities|Array|ContainsItem (LocalVariables|GetLOpenSet) _array_element))
                (Utilities|Array|Add (LocalVariables|GetLOpenSet) _array_element))))))))
  (return 0))

(fn FindPath3
  (params (Start :type My%20Tile%20Object%20Reference) (Target :type My%20Tile%20Object%20Reference))
  (bind _lcloseset (LocalVariables|GetLCloseSet))
  (bind _lopenset (LocalVariables|GetLOpenSet))
  (bind _i (LocalVariables|GetI))
  (bind _lopenset_2 (LocalVariables|GetLOpenSet))
  (LocalVariables|SetNode Start)
  (LocalVariables|SetLTarget Target)
  (bind _distance (CallFunction|GetDistance2 (LocalVariables|GetNode) (LocalVariables|GetNode)))
  (Variables|/Game/Blueprints/MyTile.MyTile_C|SetgCost (LocalVariables|GetNode) _distance)
  (bind _distance_2 (CallFunction|GetDistance2 (LocalVariables|GetNode) (LocalVariables|GetLTarget)))
  (Variables|/Game/Blueprints/MyTile.MyTile_C|SethCost (LocalVariables|GetNode) _distance_2)
  (Default|FCostCalc (LocalVariables|GetNode))
  (Utilities|Array|Add (LocalVariables|GetLOpenSet) (LocalVariables|GetNode))
  (while (or (> (Utilities|Array|Length (LocalVariables|GetLOpenSet)) 0) (< _i 100))
    (LocalVariables|SetLCurrent (Utilities|Array|Get(acopy) (LocalVariables|GetLOpenSet)))
    (Math|Integer|IncrementInt _i
      (:%20%20
        (for _index (range 1 (Utilities|Array|Length _lopenset_2))
          (if (and (or (< (Variables|/Game/Blueprints/MyTile.MyTile_C|GetfCost (Utilities|Array|Get(acopy) _lopenset_2 _index)) (Variables|/Game/Blueprints/MyTile.MyTile_C|GetfCost (LocalVariables|GetLCurrent))) (== (Variables|/Game/Blueprints/MyTile.MyTile_C|GetfCost (Utilities|Array|Get(acopy) _lopenset_2 _index)) (Variables|/Game/Blueprints/MyTile.MyTile_C|GetfCost (LocalVariables|GetLCurrent)))) (< (Variables|/Game/Blueprints/MyTile.MyTile_C|GethCost (Utilities|Array|Get(acopy) _lopenset_2 _index)) (Variables|/Game/Blueprints/MyTile.MyTile_C|GethCost (LocalVariables|GetLCurrent))))
            (LocalVariables|SetLCurrent (Utilities|Array|Get(acopy) _lopenset_2 _index))))
        (Utilities|Array|RemoveItem (LocalVariables|GetLOpenSet) (LocalVariables|GetLCurrent))
        (if (not (Utilities|Array|ContainsItem _lcloseset (LocalVariables|GetLCurrent)))
          (Utilities|Array|Add _lcloseset (LocalVariables|GetLCurrent)))
        (if (== (LocalVariables|GetLCurrent) (LocalVariables|GetLTarget))
          (return (LocalVariables|GetPAATH))
          (else
            (bind _outactors (Actor|GetAllActorsOfClass "/Game/Blueprints/MyBattleMap.MyBattleMap_C"))
            (if (Utilities|IsValid (LocalVariables|GetLCurrent))
              (bind _neighbours (Default|GetNeighbours2 (Utilities|Array|Get(acopy) _outactors) (LocalVariables|GetLCurrent)))
              (for _array_element _neighbours
                (bind _output_get (LocalVariables|SetNeighbour _array_element))
                (bind _distance_3 (CallFunction|GetDistance2 (LocalVariables|GetLCurrent) _output_get))
                (bind _output_get_2 (LocalVariables|SetMoveCost (+ (Variables|/Game/Blueprints/MyTile.MyTile_C|GetgCost (LocalVariables|GetLCurrent)) _distance_3)))
                (if (or (< _output_get_2 (Variables|/Game/Blueprints/MyTile.MyTile_C|GetgCost (LocalVariables|GetNeighbour))) (not (Utilities|Array|ContainsItem (LocalVariables|GetLOpenSet) (LocalVariables|GetNeighbour))))
                  (Variables|/Game/Blueprints/MyTile.MyTile_C|SetgCost (LocalVariables|GetNeighbour) _output_get_2)
                  (bind _distance_4 (CallFunction|GetDistance2 (LocalVariables|GetNeighbour) (LocalVariables|GetLTarget)))
                  (Variables|/Game/Blueprints/MyTile.MyTile_C|SethCost (LocalVariables|GetNeighbour) _distance_4)
                  (Default|FCostCalc (LocalVariables|GetNeighbour))
                  (Variables|/Game/Blueprints/MyTile.MyTile_C|SetParent (LocalVariables|GetNeighbour) (LocalVariables|GetLCurrent))
                  (if (not (Utilities|Array|ContainsItem _lopenset (LocalVariables|GetNeighbour)))
                    (Utilities|Array|Add _lopenset (LocalVariables|GetNeighbour)))))
              (else
                (Development|PrintString "pues es null a saber por que"))))))))
  (bind _endpath (CallFunction|RetracePath Start Target))
  (return _endpath))

(fn GetDistance2
  (params (TileA :type My%20Tile%20Object%20Reference) (TileB :type My%20Tile%20Object%20Reference))
  (bind _co_x (Variables|/Script/BattlePlanner.Tile|Getco_x TileB))
  (bind _co_ynt (Variables|/Script/BattlePlanner.Tile|Getco_ynt TileA))
  (bind _co_x_2 (Variables|/Script/BattlePlanner.Tile|Getco_x TileA))
  (bind _co_ynt_2 (Variables|/Script/BattlePlanner.Tile|Getco_ynt TileB))
  (bind _returnvalue (- _co_x_2 _co_x))
  (bind _returnvalue_2 (- _co_ynt _co_ynt_2))
  (if (< _returnvalue _returnvalue_2)
    (return _returnvalue_2)
    (else
      (return _returnvalue))))

(fn FindPath4
  (params (Start :type My%20Tile%20Object%20Reference) (Target :type My%20Tile%20Object%20Reference))
  (bind _lcloseset (LocalVariables|GetLCloseSet))
  (bind _lopenset (LocalVariables|GetLOpenSet))
  (bind _i (LocalVariables|GetI))
  (LocalVariables|SetNode Start)
  (LocalVariables|SetLTarget Target)
  (bind _distance (CallFunction|GetDistance (LocalVariables|GetNode) (LocalVariables|GetNode)))
  (Variables|/Game/Blueprints/MyTile.MyTile_C|SetgCost (LocalVariables|GetNode) _distance)
  (bind _distance_2 (CallFunction|GetDistance (LocalVariables|GetNode) (LocalVariables|GetLTarget)))
  (Variables|/Game/Blueprints/MyTile.MyTile_C|SethCost (LocalVariables|GetNode) _distance_2)
  (Default|FCostCalc (LocalVariables|GetNode))
  (Utilities|Array|Add (LocalVariables|GetLOpenSet) (LocalVariables|GetNode))
  (while (or (> (Utilities|Array|Length (LocalVariables|GetLOpenSet)) 0) (< _i 100))
    (LocalVariables|SetLCurrent (Utilities|Array|Get(acopy) (LocalVariables|GetLOpenSet)))
    (Math|Integer|IncrementInt _i
      (:%20%20
        (for _index (range 1 (Utilities|Array|LastIndex (LocalVariables|GetLOpenSet)))
          (if (and (or (< (Variables|/Game/Blueprints/MyTile.MyTile_C|GetfCost (Utilities|Array|Get(acopy) (LocalVariables|GetLOpenSet) _index)) (Variables|/Game/Blueprints/MyTile.MyTile_C|GetfCost (LocalVariables|GetLCurrent))) (== (Variables|/Game/Blueprints/MyTile.MyTile_C|GetfCost (Utilities|Array|Get(acopy) (LocalVariables|GetLOpenSet) _index)) (Variables|/Game/Blueprints/MyTile.MyTile_C|GetfCost (LocalVariables|GetLCurrent)))) (< (Variables|/Game/Blueprints/MyTile.MyTile_C|GethCost (Utilities|Array|Get(acopy) (LocalVariables|GetLOpenSet) _index)) (Variables|/Game/Blueprints/MyTile.MyTile_C|GethCost (LocalVariables|GetLCurrent))))
            (LocalVariables|SetLCurrent (Utilities|Array|Get(acopy) (LocalVariables|GetLOpenSet) _index))))
        (Utilities|Array|RemoveItem (LocalVariables|GetLOpenSet) (LocalVariables|GetLCurrent))
        (if (not (Utilities|Array|ContainsItem _lcloseset (LocalVariables|GetLCurrent)))
          (Utilities|Array|Add _lcloseset (LocalVariables|GetLCurrent)))
        (if (== (LocalVariables|GetLCurrent) (LocalVariables|GetLTarget))
          (return (LocalVariables|GetPAATH))
          (else
            (bind _outactors (Actor|GetAllActorsOfClass "/Game/Blueprints/MyBattleMap.MyBattleMap_C"))
            (if (Utilities|IsValid (LocalVariables|GetLCurrent))
              (bind _neighbours (Default|GetNeighbours2 (Utilities|Array|Get(acopy) _outactors) (LocalVariables|GetLCurrent)))
              (for _array_element _neighbours
                (bind _output_get (LocalVariables|SetNeighbour _array_element))
                (bind _distance_3 (CallFunction|GetDistance (LocalVariables|GetLCurrent) _output_get))
                (bind _output_get_2 (LocalVariables|SetMoveCost (+ (Variables|/Game/Blueprints/MyTile.MyTile_C|GetgCost (LocalVariables|GetLCurrent)) _distance_3)))
                (if (or (< _output_get_2 (Variables|/Game/Blueprints/MyTile.MyTile_C|GetgCost (LocalVariables|GetNeighbour))) (not (Utilities|Array|ContainsItem (LocalVariables|GetLOpenSet) (LocalVariables|GetNeighbour))))
                  (Variables|/Game/Blueprints/MyTile.MyTile_C|SetgCost (LocalVariables|GetNeighbour) _output_get_2)
                  (bind _distance_4 (CallFunction|GetDistance (LocalVariables|GetNeighbour) (LocalVariables|GetLTarget)))
                  (Variables|/Game/Blueprints/MyTile.MyTile_C|SethCost (LocalVariables|GetNeighbour) _distance_4)
                  (Default|FCostCalc (LocalVariables|GetNeighbour))
                  (Utilities|Array|Add (LocalVariables|GetPAATH) (LocalVariables|GetNeighbour))
                  (Variables|/Game/Blueprints/MyTile.MyTile_C|SetParent (LocalVariables|GetNeighbour) (LocalVariables|GetLCurrent))
                  (if (not (Utilities|Array|ContainsItem _lopenset (LocalVariables|GetNeighbour)))
                    (Utilities|Array|Add _lopenset (LocalVariables|GetNeighbour)))))
              (else
                (Development|PrintString "pues es null a saber por que"))))))))
  (return (LocalVariables|GetPAATH)))

(fn FindPath5
  (params (Unit :type My%20Unit%20Object%20Reference) (Target :type My%20Tile%20Object%20Reference))
  (bind _paath (LocalVariables|GetPAATH))
  (Variables|Default|SetUnit Unit)
  (bind _output_get (LocalVariables|SetLStart (Variables|/Game/Blueprints/Units/MyUnit.MyUnit_C|GetTile Unit)))
  (bind _output_get_2 (LocalVariables|SetLTarget Target))
  (bind _output_get_3 (LocalVariables|SetLCurrent _output_get))
  (bind _distance (CallFunction|GetDistance _output_get _output_get_2))
  (Variables|/Game/Blueprints/MyTile.MyTile_C|SetfCost _output_get_3 _distance)
  (while (!= (LocalVariables|GetLCurrent) (LocalVariables|GetLTarget))
    (LocalVariables|SetLCurrent_0 (LocalVariables|GetLCurrent))
    (for _array_element (Variables|/Game/Blueprints/MyTile.MyTile_C|GetNeighbours (LocalVariables|GetLCurrent))
      (bind _output_get_4 (LocalVariables|SetNeighbour _array_element))
      (bind _distance_2 (CallFunction|GetDistance _output_get_4 (LocalVariables|GetLTarget)))
      (Variables|/Game/Blueprints/MyTile.MyTile_C|SetfCost _output_get_4 _distance_2)
      (if (< (Variables|/Game/Blueprints/MyTile.MyTile_C|GetfCost (LocalVariables|GetNeighbour)) (Variables|/Game/Blueprints/MyTile.MyTile_C|GetfCost (LocalVariables|GetLCurrent_0)))
        (LocalVariables|SetLCurrent_0 _array_element)))
    (if (not (Utilities|Array|ContainsItem _paath (LocalVariables|GetLCurrent_0)))
      (Utilities|Array|Add _paath (LocalVariables|GetLCurrent_0)))
    (LocalVariables|SetLCurrent (LocalVariables|GetLCurrent_0)))
  (return (LocalVariables|GetPAATH)))

(fn GetDistance3
  (params (TileA :type My%20Tile%20Object%20Reference) (TileB :type My%20Tile%20Object%20Reference))
  (return (Math|Float|Truncate (Math|Vector|Distance(Vector) (Transformation|GetWorldLocation (Variables|/Game/Blueprints/MyTile.MyTile_C|GetStaticMesh TileA)) (Transformation|GetWorldLocation (Variables|/Game/Blueprints/MyTile.MyTile_C|GetStaticMesh TileB))))))