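; MyBattleMap is an actor that generates the battle map as a two-level grid when play begins.
; CreateMap uses a 2D grid macro around the actor's location to spawn a MyTerrainUnit at each sector center.
; Each unit receives its grid coordinates, tile row counts and tile sizes, then spawns its own tiles through SpawnTiles.
; The map also stores its overall X and Y size, derived from those dimensions.
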(event EventBeginPlay
  (CallFunction|CreateMap))

(event Collision|EventActorBeginOverlap
  (params (OtherActor :type Actor%20Object%20Reference)))

(event EventTick
  (params (DeltaSeconds :type Float%20%28single-precision%29)))

(fn ConstructionScript)

(fn CreateMap
  (bind (_current_point _total_points _0_1_phase _poly_center _x_row _y_row) (Utilities|2DGridExecutionMacroXY (* (Variables|Default|Getturows_x) (Variables|Default|Gettilesize_x)) (* (Variables|Default|Getturows_y) (Variables|Default|Gettilesize_y)) (Transformation|GetActorLocation) (Variables|Default|Getrows_x) (Variables|Default|Getrows_y))
    (:Per%20Poly%20Execution
      (bind _returnvalue (Game|SpawnActorfromClass "/Game/Blueprints/MyTerrainUnit.MyTerrainUnit_C" (Math|Transform|MakeTransform _poly_center "0, 0, 0" "1,1.000000,1") "Undefined" 0 0))
      (Variables|/Script/BattlePlanner.TerrainUnit|Setco_x _returnvalue _x_row)
      (Variables|/Script/BattlePlanner.TerrainUnit|Setco_y _returnvalue _y_row)
      (Variables|/Script/BattlePlanner.TerrainUnit|Setrows_x _returnvalue (Variables|Default|Getturows_x))
      (Variables|/Script/BattlePlanner.TerrainUnit|Setrows_y _returnvalue (Variables|Default|Getturows_y))
      (Variables|/Script/BattlePlanner.TerrainUnit|Settilesize_x _returnvalue (Variables|Default|Gettilesize_x))
      (Variables|/Script/BattlePlanner.TerrainUnit|Settilesize_y _returnvalue (Variables|Default|Gettilesize_y))
      (Variables|Default|Setsize_x (* (* (Variables|Default|Getturows_x) (Variables|Default|Getrows_x)) (Variables|Default|Gettilesize_x)))
      (Variables|Default|Setsize_y (* (* (Variables|Default|Getturows_y) (Variables|Default|Getrows_y)) (Variables|Default|Gettilesize_y)))
      (Default|SpawnTiles _returnvalue))))